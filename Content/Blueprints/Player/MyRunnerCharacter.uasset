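; Player character for a 2D runner game that creates the HUD, tracks the high score and swaps between run and jump flipbooks.
; BeginPlay loads the high score from a SaveHighScore slot and, only if that save exists, pauses the game after a brief delay; Enter unpauses.
; GameLost saves the score if it beats the high score, then quits the game.
; Tick picks the flipbook from whether the character is falling.
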(event `Key|Enter` :paused true
  (params (Key :type "Key Structure"))
  (:`Pressed`
    (`GameplayStatics.SetGamePaused` false)))

(event `self.GameLost`
  ;[1 1 1] Handle Game Lost
  (if (> (`self.Score`) (`self.Highscore`))
    (bind _output_get (set `self.Highscore` (`self.Score`)))
    (bind _returnvalue (`GameplayStatics.DoesSaveGameExist` "Save1"))
    (if _returnvalue
      (bind _returnvalue_2 (`GameplayStatics.LoadGameFromSlot` "Save1"))
      (bind _output_get_2 (set `self.SaverSubclass` _returnvalue_2))
      (bind _assave_high_score (cast `/Game/Blueprints/UI/SaveHighScore` _output_get_2))
      (set `/Game/Blueprints/UI/SaveHighScore.Highscore` _output_get _assave_high_score)
      (`GameplayStatics.SaveGameToSlot` _assave_high_score "Save1")
      (else
        (bind _returnvalue_3 (`GameplayStatics.CreateSaveGameObject` "/Game/Blueprints/UI/SaveHighScore.SaveHighScore_C"))
        (bind _output_get_3 (set `self.SaverSubclass` _returnvalue_3))
        (bind _assave_high_score_2 (cast `/Game/Blueprints/UI/SaveHighScore` _output_get_3))
        (set `/Game/Blueprints/UI/SaveHighScore.Highscore` _output_get _assave_high_score_2)
        (`GameplayStatics.SaveGameToSlot` _assave_high_score_2 "Save1"))))
  (`KismetSystemLibrary.QuitGame` null "Quit"))

(event `self.ReceiveBeginPlay`
  (bind _returnvalue (`|GenericCreateObject` "/Game/Blueprints/UI/WB_UI.WB_UI_C"))
  (`UserWidget.AddToViewport` _returnvalue 0)
  (bind _returnvalue_2 (`GameplayStatics.DoesSaveGameExist` "Save1"))
  (if _returnvalue_2
    (`KismetSystemLibrary.PrintString` "Save exists")
    (bind _returnvalue_3 (`GameplayStatics.LoadGameFromSlot` "Save1"))
    (bind _output_get (set `self.SaverSubclass` _returnvalue_3))
    (bind _assave_high_score (cast `/Game/Blueprints/UI/SaveHighScore` _output_get))
    (bind _output_get_2 (set `/Game/Blueprints/UI/SaveHighScore.Highscore` (`/Game/Blueprints/UI/SaveHighScore.Highscore` _assave_high_score) _assave_high_score))
    (set `self.Highscore` _output_get_2)
    (`KismetSystemLibrary.Delay` 0.05)
    (`GameplayStatics.SetGamePaused` true)
    (else
      (`KismetSystemLibrary.PrintString` "Save does not exist"))))

(event `self.ReceiveTick`
  (params (DeltaSeconds :type "Float (single-precision)"))
  (if (`NavMovementComponent.IsFalling` (`self.CharacterMovement`))
    (`PaperFlipbookComponent.SetFlipbook` (`self.Sprite`) "/Game/Sprite/CharacterSprites/CharacterJump.CharacterJump")
    (else
      (`PaperFlipbookComponent.SetFlipbook` (`self.Sprite`) "/Game/Sprite/CharacterSprites/CharacterRun.CharacterRun"))))

(fn `UserConstructionScript`)